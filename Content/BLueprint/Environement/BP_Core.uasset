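; BP_Core is the player's base, whose hit points drop when monsters reach it.
; A BP_Monster overlapping MonsterCollision is killed, and any remaining HP is reduced by a fixed amount.
; The new value is copied to MainGameMode and the first IngameWidget found, while Tick refreshes a TextRender readout.
; NewFunction0 is an unfinished latitude/longitude-to-position conversion that returns zeros.
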(event OnComponentBeginOverlap(MonsterCollision)
  (params (OverlappedComponent :type Primitive%20Component%20Object%20Reference) (OtherActor :type Actor%20Object%20Reference) (OtherComp :type Primitive%20Component%20Object%20Reference) (OtherBodyIndex :type Integer) (bFromSweep :type Boolean) (SweepResult :type Hit%20Result%20Structure%20%28by%20ref%29))
  (if (== (Utilities|GetClass OtherActor) "/Game/BLueprint/AI/BP_Monster.BP_Monster_C")
    (bind _asbp_monster (Utilities|Casting|CastToBP_Monster OtherActor))
    (Default|KillMonster _asbp_monster)
    (Math|Float|CompareFloat (Variables|Default|GetHitPoints) 0.0
      (:>
        (Variables|Default|SetHitPoints (- (Variables|Default|GetHitPoints) 1e+02))
        (bind _asmain_game_mode (Utilities|Casting|CastToMainGameMode (Game|GetGameMode)))
        (Variables|/Game/MainGameMode.MainGameMode_C|SetBaseHitPoints _asmain_game_mode (Variables|Default|GetHitPoints))
        (bind _foundwidgets (Widget|GetAllWidgetsOfClass "/Game/UserInterface/IngameWidget.IngameWidget_C" true))
        (Default|UpdateBaseHP (Utilities|Array|Get(acopy) _foundwidgets) (Variables|Default|GetHitPoints))))))

(event EventBeginPlay)

(event EventTick
  (params (DeltaSeconds :type Float%20%28single-precision%29))
  (Rendering|Components|TextRender|SetText (Variables|Default|GetTextRender) (Utilities|Text|ToText(Float) (Variables|Default|GetHitPoints) "HalfToEven")))

(fn ConstructionScript)

(fn NewFunction0
  (params (Long :type Float%20%28single-precision%29) (Lat :type Float%20%28single-precision%29) (Alt :type Float%20%28single-precision%29))
  (return 0.0 0.0 0.0))