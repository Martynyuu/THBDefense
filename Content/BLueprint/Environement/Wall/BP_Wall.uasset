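; BP_Wall is a wall actor built from a spline mesh that stretches from its origin toward a referenced player until it is finished.
; On BeginPlay it pins the start and runs a timeline that moves the end to the player's location, converted through the root's relative transform.
; FInischWall stops that tracking and swaps the mesh to a cube, and DestroyWall removes the actor.
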(event Custom|FInischWall
  (Components|StaticMesh|SetStaticMesh (Variables|Default|GetSplineMesh) "/Engine/EngineMeshes/Cube.Cube")
  (Timeline|Timeline_0 Stop
    (:Update
      (SplineMesh|SetEndPosition (Variables|Default|GetSplineMesh) (Math|Transform|InverseTransformLocation (Transformation|GetRelativeTransform (Variables|Default|GetDefaultSceneRoot)) (Transformation|GetWorldLocation (Variables|/Game/BLueprint/Player/PlayerPawn.PlayerPawn_C|GetDefaultSceneRoot (Variables|Default|GetPlayer%20Ref)))) true))))

(event Custom|DestroyWall
  (Actor|DestroyActor))

(event EventBeginPlay
  (SplineMesh|SetStartPosition (Variables|Default|GetSplineMesh) "0, 0, 0" true)
  (Timeline|Timeline_0 Play
    (:Update
      (SplineMesh|SetEndPosition (Variables|Default|GetSplineMesh) (Math|Transform|InverseTransformLocation (Transformation|GetRelativeTransform (Variables|Default|GetDefaultSceneRoot)) (Transformation|GetWorldLocation (Variables|/Game/BLueprint/Player/PlayerPawn.PlayerPawn_C|GetDefaultSceneRoot (Variables|Default|GetPlayer%20Ref)))) true))))

(fn ConstructionScript)