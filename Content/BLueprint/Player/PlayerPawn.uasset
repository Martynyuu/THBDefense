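; Player pawn for a location-based tower-defense style game: reads device GPS, shows coordinates on a text render and creates the in-game HUD.
; Places coin-priced towers, blocked while overlapping another tower, and toggles wall building between spawn and finish.
; Pinch touch zooms the spring arm; Android Back quits.
; GPS-to-world lerped movement exists but is disconnected in favour of debug WASD movement, with Space placing towers.
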(event OnComponentBeginOverlap(Sphere1)
  (params (OverlappedComponent :type Primitive%20Component%20Object%20Reference) (OtherActor :type Actor%20Object%20Reference) (OtherComp :type Primitive%20Component%20Object%20Reference) (OtherBodyIndex :type Integer) (bFromSweep :type Boolean) (SweepResult :type Hit%20Result%20Structure%20%28by%20ref%29))
  (if (== (Utilities|GetClass OtherActor) "/Game/BLueprint/AI/BP_Tower.BP_Tower_C")
    (Variables|Default|SetOverlappedTower OtherActor)
    (Variables|Default|SetIsOverlapBuilding? true)))

(event OnComponentEndOverlap(Sphere1)
  (params (OverlappedComponent :type Primitive%20Component%20Object%20Reference) (OtherActor :type Actor%20Object%20Reference) (OtherComp :type Primitive%20Component%20Object%20Reference) (OtherBodyIndex :type Integer))
  (if (== OtherActor (Variables|Default|GetOverlappedTower))
    (Variables|Default|SetIsOverlapBuilding? false)))

(event Custom|Place%20Tower
  (params (Type :type ENUM_DamgeTypes%20Enum :default "NewEnumerator0"))
  (bind _gamemoderef (Variables|Default|GetGamemodeRef))
  (if (>= (Variables|/Game/MainGameMode.MainGameMode_C|GetCoins _gamemoderef) 10)
    (if (not (Variables|Default|GetIsOverlapBuilding?))
      (Default|AddCoins _gamemoderef -10)
      (Game|SpawnActorfromClass "/Game/BLueprint/AI/BP_Tower.BP_Tower_C" (Transformation|GetWorldTransform (Variables|Default|GetDefaultSceneRoot)) "AlwaysSpawn" 0 Type 0)
      (Audio|PlaySound2D "/Game/Sound/SFX/Platzieren_Cue.Platzieren_Cue" 1.0 1.0 0.0 0 0))))

(event Custom|PlaceWallStart
  (bind _returnvalue (Game|SpawnActorfromClass "/Game/BLueprint/Environement/Wall/BP_Wall.BP_Wall_C" (Transformation|GetWorldTransform (Variables|Default|GetDefaultSceneRoot)) "AlwaysSpawn" 0 self 0))
  (Variables|Default|SetWallRef _returnvalue)
  (Variables|Default|SetIsWallBuilding? true))

(event Custom|PlaceWallEnd
  (Default|FInischWall (Variables|Default|GetWallRef))
  (Variables|Default|SetIsWallBuilding? false))

(event Custom|PlaceWall
  (if (Variables|Default|GetIsWallBuilding?)
    (CallFunction|PlaceWallEnd)
    (else
      (CallFunction|PlaceWallStart))))

(event Custom|SetNewPosition
  (bind _locationgps (Variables|Default|GetLocationGPS))
  (bind (_x _y) (Utilities|GPStoXYZ (.longitude _locationgps) (.latitude _locationgps) (.altitude _locationgps)))
  (bind _returnvalue (Math|Vector|MakeVector _x _y 0.0))
  (Utilities|FlowControl|Sequence
    (:then_0
      (bind _newtrack_0 (Timeline|Lerp PlayFromStart)
        (:Update
          (Transformation|SetWorldLocation (Variables|Default|GetDefaultSceneRoot) (Math|Vector|Lerp(Vector) (Variables|Default|GetLocation) (Math|Vector|MakeVector (+ (.x _returnvalue) 3.462e+06) (+ (.y _returnvalue) -1.09e+05) (+ (.z _returnvalue) 0.0)) _newtrack_0) false false))
        (:Finished
          (Variables|Default|SetLocation (Math|Vector|Lerp(Vector) (Variables|Default|GetLocation) (Math|Vector|MakeVector (+ (.x _returnvalue) 3.462e+06) (+ (.y _returnvalue) -1.09e+05) (+ (.z _returnvalue) 0.0)) _newtrack_0)))))
    (:then_1
      (Utilities|FlowControl|DoOnce false
        (:Completed
          (Variables|Default|SetLocation (Transformation|GetWorldLocation (Variables|Default|GetDefaultSceneRoot))))))))

(event EventBeginPlay
  ;[1 1 1] Begin Play
  (bind _asmain_game_mode (Utilities|Casting|CastToMainGameMode (Game|GetGameMode)))
  (Variables|Default|SetGamemodeRef _asmain_game_mode)
  (bind _returnvalue (Class|LocationServices|StartLocationServices))
  (bind _returnvalue_2 (UserInterface|CreateWidget "/Game/UserInterface/IngameWidget.IngameWidget_C"))
  (Variables|Default|SetWidgetRef _returnvalue_2)
  (Variables|/Game/UserInterface/IngameWidget.IngameWidget_C|SetPlayerPawnRef _returnvalue_2 self)
  (UserInterface|Viewport|AddtoViewport _returnvalue_2 1)
  (if _returnvalue
    (Actor|Tick|SetActorTickEnabled true)
    (else
      (Rendering|Components|TextRender|SetText (Variables|Default|GetTextRender) (Utilities|Text|MakeLiteralText "No   
GPS")))))

(event EventTick
  (params (DeltaSeconds :type Float%20%28single-precision%29))
  ;[1 1 1] Event Tick
  (Rendering|Components|TextRender|SetText (Variables|Default|GetTextRender) (Utilities|Text|ToText(String) (Utilities|String|Append "" "Long.: " (Utilities|String|ToString(Float) (.longitude (Variables|Default|GetLocationGPS))) "  
Lat.:" (Utilities|String|ToString(Float) (.latitude (Variables|Default|GetLocationGPS))) " 
Alt.:" (Utilities|String|ToString(Vector) (Variables|Default|GetLocation)))))
  (bind _returnvalue (Class|LocationServices|GetLastKnownLocation))
  (Variables|Default|SetLocationGPS _returnvalue))

(event Input|AxisEvents|InputAxisPinch
  (params (AxisValue :type Float%20%28single-precision%29))
  ;[1 1 1] Pinch Zoom
)

(event Input|KeyboardEvents|X
  (params (Key :type Key%20Structure)))

(event Input|KeyboardEvents|W
  (params (Key :type Key%20Structure))
  ;[1 0.04746 0.1371] Debug
  (:Pressed
    (Timeline|Timeline_0 Play
      (:Update
        (Transformation|AddActorWorldOffset "5.000000, 0, 0"))))
  (:Released
    (Timeline|Timeline_0 Stop)))

(event Input|KeyboardEvents|AndroidBack
  (params (Key :type Key%20Structure))
  (:Pressed
    (Game|QuitGame 0 "Quit" false)))

(event Input|KeyboardEvents|S
  (params (Key :type Key%20Structure))
  ;[1 0.04746 0.1371] Debug
  (:Pressed
    (Timeline|Timeline_1 Play
      (:Update
        (Transformation|AddActorWorldOffset "-5.000000, 0, 0"))))
  (:Released
    (Timeline|Timeline_1 Stop)))

(event Input|KeyboardEvents|A
  (params (Key :type Key%20Structure))
  ;[1 0.04746 0.1371] Debug
  (:Pressed
    (Timeline|Timeline_2 Play
      (:Update
        (Transformation|AddActorWorldOffset "0.000000,-5.000000, 0"))))
  (:Released
    (Timeline|Timeline_2 Stop)))

(event Input|KeyboardEvents|D
  (params (Key :type Key%20Structure))
  ;[1 0.04746 0.1371] Debug
  (:Pressed
    (Timeline|Timeline_3 Play
      (:Update
        (Transformation|AddActorWorldOffset "0.000000,5.000000, 0"))))
  (:Released
    (Timeline|Timeline_3 Stop)))

(event Input|KeyboardEvents|SpaceBar
  (params (Key :type Key%20Structure))
  ;[1 0.04746 0.1371] Debug
  (:Pressed
    (if (not (Variables|Default|GetIsOverlapBuilding?))
      (CallFunction|PlaceTower "NewEnumerator0"))))

(event Input|TouchEvents|InputTouch
  (params (Location :type Vector) (FingerIndex :type ETouchIndex%20Enum))
  (bind _springarm (Variables|Default|GetSpringArm))
  ;[1 1 1] Pinch Zoom
  (:Moved
    (if (Utilities|Enum|Equal(Enum) FingerIndex "Touch2")
      (if (> (stale Input|AxisEvents|InputAxisPinch AxisValue) 1.1)
        (Math|Float|CompareFloat (- (Variables|/Script/Engine.SpringArmComponent|GetTargetArmLength _springarm) 15.0) 0.0
          (:>
            (Variables|/Script/Engine.SpringArmComponent|SetTargetArmLength _springarm (- (Variables|/Script/Engine.SpringArmComponent|GetTargetArmLength _springarm) 15.0))))
        (elif (< (stale Input|AxisEvents|InputAxisPinch AxisValue) 0.9)
          (Math|Float|CompareFloat (+ (Variables|/Script/Engine.SpringArmComponent|GetTargetArmLength _springarm) 15.0) 1.2e+04
            (:<
              (Variables|/Script/Engine.SpringArmComponent|SetTargetArmLength _springarm (+ (Variables|/Script/Engine.SpringArmComponent|GetTargetArmLength _springarm) 15.0)))))))))

(fn ConstructionScript)