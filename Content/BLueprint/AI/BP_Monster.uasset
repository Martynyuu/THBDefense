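; BP_Monster is an enemy that takes damage and, on death, awards a coin through the game mode, plays a sound and destroys itself.
; An overlap sphere tracks nearby towers and walls.
; Tick compares the mesh's absolute X/Y to a saved location, displaying the Y difference.
; A difference over 200 feeds a 10-second retriggerable delay, then destroys tracked buildings and the monster; otherwise the saved location updates.
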(event OnComponentBeginOverlap(Sphere)
  (params (OverlappedComponent :type Primitive%20Component%20Object%20Reference) (OtherActor :type Actor%20Object%20Reference) (OtherComp :type Primitive%20Component%20Object%20Reference) (OtherBodyIndex :type Integer) (bFromSweep :type Boolean) (SweepResult :type Hit%20Result%20Structure%20%28by%20ref%29))
  (bind _asbp_tower (Utilities|Casting|CastToBP_Tower OtherActor)
    (:then
      (Utilities|Array|AddUnique (Variables|Default|GetTowers) _asbp_tower)
      (Development|PrintString "Building"))
    (:CastFailed
      (bind _asbp_wall (Utilities|Casting|CastToBP_Wall OtherActor))
      (Utilities|Array|AddUnique (Variables|Default|GetWalls) _asbp_wall)
      (Development|PrintString "Wall"))))

(event OnComponentEndOverlap(Sphere)
  (params (OverlappedComponent :type Primitive%20Component%20Object%20Reference) (OtherActor :type Actor%20Object%20Reference) (OtherComp :type Primitive%20Component%20Object%20Reference) (OtherBodyIndex :type Integer))
  (bind _walls (Variables|Default|GetWalls))
  (bind _towers (Variables|Default|GetTowers))
  (bind _asbp_tower (Utilities|Casting|CastToBP_Tower OtherActor)
    (:then
      (Utilities|Array|RemoveItem (Variables|Default|GetTowers) _asbp_tower)
      (Utilities|Array|Resize _towers (Utilities|Array|Length _towers))
      (Development|PrintString "Building" true true "(R=1.000000,G=0.126577,B=0.000000,A=1.000000)"))
    (:CastFailed
      (bind _asbp_wall (Utilities|Casting|CastToBP_Wall OtherActor))
      (Utilities|Array|RemoveItem _walls _asbp_wall)
      (Utilities|Array|Resize (Variables|Default|GetWalls) (Utilities|Array|Length _walls))
      (Development|PrintString "Wall" true true "(R=1.000000,G=0.195490,B=0.025443,A=1.000000)"))))

(event Custom|KillMonster
  (Actor|DestroyActor))

(event Custom|ApplyDamage
  (params (IncomingDamage :type Float%20%28single-precision%29))
  (if (> IncomingDamage 0.0)
    (bind _output_get (Variables|Default|SetHealth (- (Variables|Default|GetHealth) IncomingDamage)))
    (if (<= _output_get 0.0)
      (Default|AddCoins (Variables|Default|GetGameModeRef) 1)
      (Audio|PlaySound2D "/Game/Sound/SFX/Coins.Coins" 1.0 1.0 0.0 0 0)
      (CallFunction|KillMonster))))

(event Custom|DestroyBuildingsInRange
  (bind _towers (Variables|Default|GetTowers))
  (bind _walls (Variables|Default|GetWalls))
  (for _array_element _towers
    (Default|DestroyTower _array_element))
  (Utilities|Array|Clear _towers)
  (for _array_element_2 _walls
    (Default|DestroyWall _array_element_2))
  (Utilities|Array|Clear _walls)
  (Actor|DestroyActor))

(event EventBeginPlay
  (bind _asmain_game_mode (Utilities|Casting|CastToMainGameMode (Game|GetGameMode)))
  (Variables|Default|SetGameModeRef _asmain_game_mode))

(event Collision|EventActorBeginOverlap
  (params (OtherActor :type Actor%20Object%20Reference)))

(event EventTick
  (params (DeltaSeconds :type Float%20%28single-precision%29))
  (bind _mesh (Variables|Character|GetMesh))
  (bind _mesh_2 (Variables|Character|GetMesh))
  (bind _returnvalue (Transformation|GetWorldLocation _mesh))
  (bind _returnvalue_2 (Transformation|GetWorldLocation _mesh_2))
  (Rendering|Components|TextRender|SetText (Variables|Default|GetTextRender) (Utilities|Text|ToText(Float) (- (Math|Float|Absolute(Float) (.y _returnvalue)) (Math|Float|Absolute(Float) (.y (Variables|Default|GetLastLocation)))) "HalfToEven"))
  (Utilities|FlowControl|Sequence
    (:then_0
      (if (or (> (- (Math|Float|Absolute(Float) (.x _returnvalue)) (Math|Float|Absolute(Float) (.x (Variables|Default|GetLastLocation)))) 2e+02) (> (- (Math|Float|Absolute(Float) (.y _returnvalue)) (Math|Float|Absolute(Float) (.y (Variables|Default|GetLastLocation)))) 2e+02))
        (Utilities|FlowControl|RetriggerableDelay 1e+01)
        (CallFunction|DestroyBuildingsinRange)
        (else
          (Variables|Default|SetLastLocation _returnvalue_2))))
    (:then_1
      (Utilities|FlowControl|DoOnce false
        (:Completed
          (Variables|Default|SetLastLocation _returnvalue_2))))))

(fn ConstructionScript)