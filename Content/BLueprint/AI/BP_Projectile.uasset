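; BP_Projectile is a homing projectile that damages BP_Monster actors.
; On BeginPlay it sets movement speed and homing target, then switches mesh and particle template by element (Plasma, Fire, Ice), with the switch input shown as Ice.
; It destroys itself if the target is invalid at spawn or on any Tick, or after its box overlaps a monster and applies damage.
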(event OnComponentBeginOverlap(Box)
  (params (OverlappedComponent :type Primitive%20Component%20Object%20Reference) (OtherActor :type Actor%20Object%20Reference) (OtherComp :type Primitive%20Component%20Object%20Reference) (OtherBodyIndex :type Integer) (bFromSweep :type Boolean) (SweepResult :type Hit%20Result%20Structure%20%28by%20ref%29))
  (bind _asbp_monster (Utilities|Casting|CastToBP_Monster OtherActor))
  (Default|ApplyDamage _asbp_monster (Variables|Default|GetProjectileDamage))
  (Actor|DestroyActor))

(event EventBeginPlay
  (bind _projectilemovement (Variables|Default|GetProjectileMovement))
  (bind _homingtarget (Variables|Default|GetHomingTarget))
  (bind _projectilemesh (Variables|Default|GetProjectileMesh))
  (bind _particlesystem (Variables|Default|GetParticleSystem))
  (bind _output_get (Variables|/Script/Engine.ProjectileMovementComponent|SetInitialSpeed _projectilemovement (Variables|Default|GetSpeed)))
  (Variables|/Script/Engine.ProjectileMovementComponent|SetMaxSpeed _projectilemovement _output_get)
  (Utilities|IsValid _homingtarget
    (:Is%20Valid
      (Variables|/Script/Engine.ProjectileMovementComponent|SetHomingTargetComponent _projectilemovement _homingtarget)
      (switch Utilities|FlowControl|Switch|SwitchonENUM_DamgeTypes "NewEnumerator5"
        (:NewEnumerator0
          (Components|StaticMesh|SetStaticMesh _projectilemesh "/Game/BLueprint/Environement/ProjectileFire_Kugel.ProjectileFire_Kugel")
          (Effects|Components|ParticleSystem|SetTemplate _particlesystem "/Game/AdvancedMagicFX13/Particles/P_ky_burstBall1.P_ky_burstBall1"))
        (:NewEnumerator2
          (Components|StaticMesh|SetStaticMesh _projectilemesh "/Game/BLueprint/Environement/ProjectileFire_Kugel.ProjectileFire_Kugel")
          (Effects|Components|ParticleSystem|SetTemplate _particlesystem "/Game/AdvancedMagicFX13/Particles/P_ky_cutter2.P_ky_cutter2")
          (Transformation|AddLocalRotation _particlesystem "90.000000,0.000000,90.000000" false false))
        (:NewEnumerator5
          (Components|StaticMesh|SetStaticMesh _projectilemesh "/Game/BLueprint/Environement/ProjectileIce_Platonischer_Körper_1.ProjectileIce_Platonischer_Körper_1")
          (Effects|Components|ParticleSystem|SetTemplate _particlesystem "/Game/AdvancedMagicFX13/Particles/P_ky_stabShot.P_ky_stabShot"))))
    (:Is%20Not%20Valid
      (Actor|DestroyActor))))

(event Collision|EventActorBeginOverlap
  (params (OtherActor :type Actor%20Object%20Reference)))

(event EventTick
  (params (DeltaSeconds :type Float%20%28single-precision%29))
  (Utilities|IsValid (Variables|Default|GetHomingTarget)
    (:Is%20Not%20Valid
      (Actor|DestroyActor))))

(fn ConstructionScript)