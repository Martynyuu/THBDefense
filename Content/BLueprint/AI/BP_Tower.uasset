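; BP_Tower is a tower that fires homing projectiles at monsters inside its range.
; BeginPlay labels its damage type, sets fixed base and head meshes, and sizes the detection sphere to TowerRange; the per-type mesh switch assigns only None.
; Sphere overlaps maintain the list of monsters in range.
; Every Tick, with no cooldown, it spawns a BP_Projectile homing on the list's last monster, passing speed and damage type.
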(event OnComponentBeginOverlap(Sphere)
  (params (OverlappedComponent :type Primitive%20Component%20Object%20Reference) (OtherActor :type Actor%20Object%20Reference) (OtherComp :type Primitive%20Component%20Object%20Reference) (OtherBodyIndex :type Integer) (bFromSweep :type Boolean) (SweepResult :type Hit%20Result%20Structure%20%28by%20ref%29))
  (bind _enemyinrange (Variables|Default|GetEnemyInRange))
  (Development|PrintString (Utilities|GetDisplayName OtherActor))
  (bind _asbp_monster (Utilities|Casting|CastToBP_Monster OtherActor))
  (Utilities|Array|AddUnique _enemyinrange _asbp_monster)
  (Variables|Default|SetEnemyCountInRange (Utilities|Array|Length _enemyinrange)))

(event OnComponentEndOverlap(Sphere)
  (params (OverlappedComponent :type Primitive%20Component%20Object%20Reference) (OtherActor :type Actor%20Object%20Reference) (OtherComp :type Primitive%20Component%20Object%20Reference) (OtherBodyIndex :type Integer))
  (bind _enemyinrange (Variables|Default|GetEnemyInRange))
  (bind _asbp_monster (Utilities|Casting|CastToBP_Monster OtherActor))
  (Utilities|Array|RemoveItem _enemyinrange _asbp_monster)
  (Utilities|Array|Resize _enemyinrange (Utilities|Array|Length _enemyinrange)))

(event EventBeginPlay
  (bind _damgetype (Variables|Default|GetDamgeType))
  (Rendering|Components|TextRender|SetText (Variables|Default|GetType) (Utilities|Text|ToText(String) (Utilities|String|EnumtoString _damgetype)))
  (switch Utilities|FlowControl|Switch|SwitchonENUM_DamgeTypes _damgetype
    (:NewEnumerator0
      (Variables|Default|SetTowerHeadMesh 0)
      (Variables|Default|SetTowerHeadMesh 0))
    (:NewEnumerator1
      (Variables|Default|SetTowerHeadMesh 0)
      (Variables|Default|SetTowerHeadMesh 0))
    (:NewEnumerator2
      (Variables|Default|SetTowerHeadMesh 0)
      (Variables|Default|SetTowerHeadMesh 0))
    (:NewEnumerator3
      (Variables|Default|SetTowerHeadMesh 0)
      (Variables|Default|SetTowerHeadMesh 0))
    (:NewEnumerator4
      (Variables|Default|SetTowerHeadMesh 0)
      (Variables|Default|SetTowerHeadMesh 0))
    (:NewEnumerator5
      (Variables|Default|SetTowerHeadMesh 0)
      (Variables|Default|SetTowerHeadMesh 0)))
  (Components|StaticMesh|SetStaticMesh (Variables|Default|GetBase) "/Game/BLueprint/Environement/Tower2fix.Tower2fix")
  (Components|StaticMesh|SetStaticMesh (Variables|Default|GetHead) "/Engine/EditorMeshes/ArcadeEditorSphere.ArcadeEditorSphere")
  (Components|Sphere|SetSphereRadius (Variables|Default|GetSphere) (Variables|Default|GetTowerRange) true))

(event EventTick
  (params (DeltaSeconds :type Float%20%28single-precision%29))
  (bind _enemyinrange (Variables|Default|GetEnemyInRange))
  (bind _arrow (Variables|Default|GetArrow))
  (bind _returnvalue (Transformation|GetWorldTransform _arrow))
  (if (> (Utilities|Array|Length (Variables|Default|GetEnemyInRange)) 0)
    (bind _output_get (Variables|Default|SetTargetEnemy (Utilities|Array|Get(acopy) _enemyinrange (Utilities|Array|LastIndex _enemyinrange))))
    (Utilities|IsValid _output_get
      (:Is%20Valid
        (Game|SpawnActorfromClass "/Game/BLueprint/AI/BP_Projectile.BP_Projectile_C" (Math|Transform|MakeTransform (.location _returnvalue) (.rotation _returnvalue) "10.000000,10.000000,10.000000") "AlwaysSpawn" 0 (Variables|Default|GetProjectileSpeed) (Variables|Default|GetDamgeType) (Variables|/Game/BLueprint/AI/BP_Monster.BP_Monster_C|GetScene (Variables|Default|GetTargetEnemy)) 0)))))

(fn ConstructionScript)